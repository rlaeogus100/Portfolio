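; GA_MeleeBase is a Gameplay Ability for melee attacks that applies damage to targets.
; On activation it commits, then plays the attack montage and waits for a Health.Damage gameplay event.
; When the event arrives, it prints a debug string and applies GE_GetDamage to the event payload's target data.
; The ability ends when the montage blends out, is interrupted or is cancelled.
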(event `self.K2_ActivateAbility`
  (bind _returnvalue (`self.K2_CommitAbility`))
  (if _returnvalue
    (`AbilityTask_PlayMontageAndWait.CreatePlayMontageAndWaitProxy` "None" (`self.ToPlayMontage`)
      (:`then`
        (bind (_asynctaskproxy _payload) (`AbilityTask_WaitGameplayEvent.WaitGameplayEvent` (struct :`TagName` "Health.Damage") null)
          (:`EventReceived`
            (`KismetSystemLibrary.PrintString` "asdfsadf")
            (`self.BP_ApplyGameplayEffectToTarget` (`.TargetData` (break `GameplayEventData` _payload)) "/Game/BluePrint/GAS/GE_GetDamage.GE_GetDamage_C"))))
      (:`OnBlendOut`
        (`self.K2_EndAbility` :!label _label))
      (:`OnInterrupted`
        (goto _label))
      (:`OnCancelled`
        (goto _label)))))
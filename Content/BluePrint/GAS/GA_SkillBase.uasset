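; Base Gameplay Ability for skills that plays a montage and spawns an actor carrying damage.
; After committing, it starts the montage and immediately spawns the actor class held in a variable just ahead of the owner, facing the same way.
; The spawned actor receives an outgoing GE_GetDamage effect spec, and its spawn transform is printed for debugging.
; The ability ends on montage blend out, interrupt or cancel, with no end path if commit fails.
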(event `self.K2_ActivateAbility`
  (bind _returnvalue (`self.GetOwningActorFromActorInfo`))
  (bind _returnvalue_2 (`Actor.K2_GetActorRotation` _returnvalue))
  (bind _returnvalue_3 (+ (* (`Actor.GetActorForwardVector` _returnvalue) 100.0) (`Actor.K2_GetActorLocation` _returnvalue)))
  (bind _returnvalue_4 (`self.K2_CommitAbility`))
  (if _returnvalue_4
    (`AbilityTask_PlayMontageAndWait.CreatePlayMontageAndWaitProxy` "None" (`self.ToPlayMontage`)
      (:`then`
        (`|SpawnActorFromClass` (`self.Class`) (`KismetMathLibrary.MakeTransform` _returnvalue_3 _returnvalue_2) "Undefined" "OverrideRootScale" _returnvalue (`AbilitySystemComponent.MakeOutgoingSpec` :`self` (`AbilitySystemBlueprintLibrary.GetAbilitySystemComponent` _returnvalue) :`GameplayEffectClass` "/Game/BluePrint/GAS/GE_GetDamage.GE_GetDamage_C") (`Actor.Instigator` _returnvalue))
        (`KismetSystemLibrary.PrintString` (`KismetStringLibrary.Conv_RotatorToString` _returnvalue_2))
        (`KismetSystemLibrary.PrintString` (`KismetStringLibrary.Conv_VectorToString` _returnvalue_3)))
      (:`OnBlendOut`
        (`self.K2_EndAbility` :!label _label))
      (:`OnInterrupted`
        (goto _label))
      (:`OnCancelled`
        (goto _label)))))
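; Base gameplay ability for character skills that plays a montage and spawns a skill actor carrying element-based damage.
; After committing, it starts the montage and immediately, on authority only, picks a damage effect spec from the BP_Character's Element (None, Fire, Aqua or Lightning).
; The configurable actor class spawns ahead of and above the owner, receiving that spec.
; The ability ends when the montage blends out, is interrupted or is cancelled.
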(event `self.K2_ActivateAbility`
  (bind _returnvalue (`self.GetOwningActorFromActorInfo`))
  (bind _returnvalue_2 (`AbilitySystemBlueprintLibrary.GetAbilitySystemComponent` _returnvalue))
  (bind (_returnvalue_x _returnvalue_y _returnvalue_z) (`KismetMathLibrary.BreakVector` (+ (* (`Actor.GetActorForwardVector` _returnvalue) 100.0) (`Actor.K2_GetActorLocation` _returnvalue))))
  (bind _returnvalue_3 (`self.K2_CommitAbility`))
  (if _returnvalue_3
    (`AbilityTask_PlayMontageAndWait.CreatePlayMontageAndWaitProxy` "None" (`self.ToPlayMontage`)
      (:`then`
        (bind _asbp_character (cast `/Game/BluePrint/Character/BP_Character` _returnvalue))
        (if (`Actor.HasAuthority` _asbp_character)
          (switch `EElementEnum` (`SharedCharacter.Element` _asbp_character)
            (:`None`
              (set `self.Gameplay Effect Spec Handle` (`AbilitySystemComponent.MakeOutgoingSpec` :`self` _returnvalue_2 :`GameplayEffectClass` "/Game/BluePrint/GAS/GE_GetDamage.GE_GetDamage_C")))
            (:`Fire`
              (set `self.Gameplay Effect Spec Handle` (`AbilitySystemComponent.MakeOutgoingSpec` :`self` _returnvalue_2 :`GameplayEffectClass` "/Game/BluePrint/GAS/ElementDamage/GE_FireDamage.GE_FireDamage_C")))
            (:`Aqua`
              (set `self.Gameplay Effect Spec Handle` (`AbilitySystemComponent.MakeOutgoingSpec` :`self` _returnvalue_2 :`GameplayEffectClass` "/Game/BluePrint/GAS/ElementDamage/GE_AquaDamage.GE_AquaDamage_C")))
            (:`Lightning`
              (set `self.Gameplay Effect Spec Handle` (`AbilitySystemComponent.MakeOutgoingSpec` :`self` _returnvalue_2 :`GameplayEffectClass` "/Game/BluePrint/GAS/ElementDamage/GE_LightningDamage.GE_LightningDamage_C"))))
          (`|SpawnActorFromClass` (`self.Class`) (`KismetMathLibrary.MakeTransform` (`KismetMathLibrary.MakeVector` _returnvalue_x _returnvalue_y (+ _returnvalue_z 90.0)) (`Actor.K2_GetActorRotation` (`self.GetOwningActorFromActorInfo`))) "Undefined" "OverrideRootScale" _returnvalue (`self.Gameplay Effect Spec Handle`) (`Actor.Instigator` _returnvalue))))
      (:`OnBlendOut`
        (`self.K2_EndAbility` :!label _label))
      (:`OnInterrupted`
        (goto _label))
      (:`OnCancelled`
        (goto _label)))))
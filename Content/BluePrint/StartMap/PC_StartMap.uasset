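; Player controller for the start map that lets the player host or join a multiplayer session.
; BeginPlay switches to UI-only input with a visible, unlocked mouse cursor.
; StartServer adds a NewWidgetBlueprint to the viewport and opens TopDownExampleMap as a listen server.
; ConnectServer adds the same widget, then travels to the passed LevelName through Open Level by name, with no options.
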(event `self.ReceiveBeginPlay`
  (`WidgetBlueprintLibrary.SetInputMode_UIOnlyEx` self null)
  (set `self.bShowMouseCursor` true))

(event `StartServer`
  (bind _returnvalue (`|CreateWidget` "/Game/BluePrint/StartMap/NewWidgetBlueprint.NewWidgetBlueprint_C"))
  (`UserWidget.AddToViewport` _returnvalue 0)
  (`GameplayStatics.OpenLevelBySoftObjectPtr` "/Game/TopDownBP/Maps/TopDownExampleMap.TopDownExampleMap" true "listen"))

(event `ConnectServer`
  (params (LevelName :type Name))
  (bind _returnvalue (`|CreateWidget` "/Game/BluePrint/StartMap/NewWidgetBlueprint.NewWidgetBlueprint_C"))
  (`UserWidget.AddToViewport` _returnvalue 0)
  (`GameplayStatics.OpenLevel` LevelName))

(fn `UserConstructionScript`)
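; Behavior tree decorator that checks whether the AI-controlled pawn currently owns any of a configured set of gameplay tags.
; The condition check loops over the Tag array and compares each entry against the owned tags on the pawn's Ability System Component.
; It returns true when at least one tag matches, and the comparison only runs for a valid pawn.
; The AI tick event is empty.
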(event `self.ReceiveTickAI`
  (params (OwnerController :type "AIController Object Reference") (ControlledPawn :type "Pawn Object Reference") (DeltaSeconds :type "Float (single-precision)")))

(fn `PerformConditionCheckAI`
  (params (OwnerController :type "AIController Object Reference") (ControlledPawn :type "Pawn Object Reference"))
  (returns (ReturnValue :type Boolean))
  (if (`KismetSystemLibrary.IsValid` ControlledPawn)
    (set `self.Boolean` false)
    (for _array_element (`self.Tag`)
      (bind _case_0_true (`|MultiCompareGameplayTagContainerSingleTags` _array_element (`GameplayTagAssetInterface.GetOwnedGameplayTags` (`AbilitySystemBlueprintLibrary.GetAbilitySystemComponent` ControlledPawn))))
      (if _case_0_true
        (set `self.Boolean` _case_0_true)))
    (return (`self.Boolean`))))
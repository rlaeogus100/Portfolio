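; Troll enemy Blueprint that reacts to seeing a pawn through PawnSensing and hands it to its AI as a target.
; If the Blackboard's TargetActor is empty, it stores the seen pawn, switches the State enum and activates Gameplay Ability System abilities by tag.
; BeginPlay prints whether an AI controller is valid, and a PrintHealth event prints current health, both as debug output.
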(event `self.ReceiveBeginPlay`
  (`KismetSystemLibrary.PrintString` (`KismetStringLibrary.Conv_BoolToString` (`KismetSystemLibrary.IsValid` (`AIBlueprintHelperLibrary.GetAIController` self)))))

(event `self.PawnSensing.OnSeePawn`
  (params (Pawn :type "Pawn Object Reference"))
  (bind _returnvalue (`AIBlueprintHelperLibrary.GetBlackboard` null))
  (if (== (`BlackboardComponent.GetValueAsObject` _returnvalue "TargetActor") null)
    (`BlackboardComponent.SetValueAsObject` _returnvalue "TargetActor" Pawn)
    (`BlackboardComponent.SetValueAsEnum` (`AIBlueprintHelperLibrary.GetBlackboard` null) "State" (enumliteral `/Game/BluePrint/Enemy/EnemyState` "NewEnumerator1"))
    (`AbilitySystemComponent.TryActivateAbilitiesByTag` (`self.AbilitySystemComp`) (`self.Gameplay Tag Container`) true)))

(event `PrintHealth`
  (bind _returnvalue (`self.GetHealth`))
  (`KismetSystemLibrary.PrintString` (`KismetStringLibrary.Conv_DoubleToString` _returnvalue)))

(fn `UserConstructionScript`)
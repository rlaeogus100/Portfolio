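; Enemy spawner Blueprint that creates an AI enemy when a BP_Character begins overlapping it.
; Spawning runs only on the authority, with a coin flip choosing Enemy_Boss or the configurable SpawnPawnClass (logged as a Troll).
; Either pawn receives the same BehaviorTree and appears at a random horizontal offset around the spawner at its height.
; Nothing disables the trigger, so every new overlap spawns again.
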(event `self.ReceiveBeginPlay`)

(event `self.ReceiveActorBeginOverlap`
  (params (OtherActor :type "Actor Object Reference"))
  (bind (_returnvalue_x _returnvalue_y _returnvalue_z) (`KismetMathLibrary.BreakVector` (`self.K2_GetActorLocation`)))
  (bind _returnvalue (`KismetMathLibrary.RandomFloatInRange` -1000.0 1000.0))
  (bind _behavior_tree (`self.Behavior Tree`))
  (bind _returnvalue_2 (+ _returnvalue_x _returnvalue))
  (bind _returnvalue_3 (+ _returnvalue_y _returnvalue))
  (cast `/Game/BluePrint/Character/BP_Character` OtherActor)
  (`/Engine/EditorBlueprintResources/ActorMacros.Switch Has Authority`
    (:`Authority`
      (if (`self.HasAuthority`)
        (if (>= (`KismetMathLibrary.RandomFloat`) 0.5)
          (`AIBlueprintHelperLibrary.SpawnAIFromClass` "/Game/BluePrint/Enemy/Enemy_Boss.Enemy_Boss_C" _behavior_tree (`KismetMathLibrary.MakeVector` _returnvalue_2 _returnvalue_3 _returnvalue_z) (struct) true null)
          (`KismetSystemLibrary.PrintString` "Spawn Boss")
          (else
            (`AIBlueprintHelperLibrary.SpawnAIFromClass` (`self.Spawn Pawn Class`) _behavior_tree (`KismetMathLibrary.MakeVector` _returnvalue_2 _returnvalue_3 _returnvalue_z) (struct) true null)
            (`KismetSystemLibrary.PrintString` "Spawn Troll")))))))

(fn `UserConstructionScript`)
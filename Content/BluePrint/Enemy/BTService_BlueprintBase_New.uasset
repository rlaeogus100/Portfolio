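; Enemy behavior tree service that drops the current target once it is too far away by path distance.
; Each AI tick, it reads TargetActor from the blackboard as a BP_Character and measures the path length from the pawn to it.
; When that length exceeds TargetLength, it sets State to the first enemy state and clears TargetActor.
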(event `self.ReceiveTickAI`
  (params (OwnerController :type "AIController Object Reference") (ControlledPawn :type "Pawn Object Reference") (DeltaSeconds :type "Float (single-precision)"))
  (bind _returnvalue (`AIBlueprintHelperLibrary.GetBlackboard` ControlledPawn))
  (bind _asbp_character (cast `/Game/BluePrint/Character/BP_Character` (`BlackboardComponent.GetValueAsObject` _returnvalue "TargetActor")))
  (if (not (<= (`NavigationSystemV1.GetPathLength` (`Actor.K2_GetActorLocation` ControlledPawn) (`Actor.K2_GetActorLocation` _asbp_character) null null) (`self.TargetLength`)))
    (`BlackboardComponent.SetValueAsEnum` _returnvalue "State" (enumliteral `/Game/BluePrint/Enemy/EnemyState` "NewEnumerator0"))
    (`BlackboardComponent.SetValueAsObject` _returnvalue "TargetActor" null)))
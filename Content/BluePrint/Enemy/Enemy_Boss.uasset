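; Boss enemy Blueprint that extends the enemy death flow to notify the player HUD when the boss dies.
; Death calls DeathToServer, then relays BossDeathToServer to BossDeathToMulticast, named as a server-to-multicast chain.
; After a two-second delay, the multicast event casts player controller 0's HUD to PlayerHUD and calls its BossDeath.
; BeginPlay, overlap and Tick are disabled stubs, and construction only calls the parent.
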(event `self.Death`
  ;[1 1 1] 보스 죽음
  (`self.DeathToServer`)
  (`self.BossDeathToServer`))

(event `BossDeathToServer`
  ;[1 1 1] 보스 죽음
  (`self.BossDeathToMulticast`))

(event `BossDeathToMulticast`
  ;[1 1 1] 보스 죽음
  (`KismetSystemLibrary.Delay` 2.0)
  (bind _asplayer_controller (cast `/Game/BluePrint/Character/PlayerController` (`GameplayStatics.GetPlayerController` 0)))
  (bind _asplayer_hud (cast `/Game/BluePrint/Character/PlayerHUD` (`PlayerController.GetHUD` _asplayer_controller)))
  (`/Game/BluePrint/Character/PlayerHUD.BossDeath` _asplayer_hud))

(fn `UserConstructionScript`
  (`parent.UserConstructionScript`))
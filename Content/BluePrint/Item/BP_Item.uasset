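; World item pickup actor that shows its name on a widget bar and can be collected by clicking it.
; On BeginPlay it loads the Sword row from ItemTable if no item is set, otherwise applies the item's static mesh, then passes the name to the widget.
; A click within range of the player character hands the item to the player controller's ItemGet, and the actor destroys itself on success.
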(event `self.ReceiveBeginPlay`
  (bind (_itemobject_itemname _itemobject_itemstaticmesh) (break `/Game/BluePrint/Inventory/ItemStruct` (`self.ItemObject`)))
  (bind _itemobject_itemname_2 (break `/Game/BluePrint/Inventory/ItemStruct` (`self.ItemObject`)))
  (if (== _itemobject_itemname "None")
    (bind _returnvalue (`|GetDataTableRow` "/Game/BluePrint/Inventory/ItemTable.ItemTable" "Sword")
      (:`then`
        (set `self.ItemObject` _returnvalue)))
    (else
      (`StaticMeshComponent.SetStaticMesh` (`self.staticMesh`) _itemobject_itemstaticmesh)))
  (bind _asitem_name_broadcast (cast `/Game/BluePrint/Item/ItemNameBroadcast` (`WidgetComponent.GetUserWidgetObject` (`self.ItemNameBar`))))
  (set `/Game/BluePrint/Item/ItemNameBroadcast.ItemName` (`KismetTextLibrary.Conv_NameToText` _itemobject_itemname_2) _asitem_name_broadcast))

(event `self.ReceiveActorOnClicked`
  (params (ButtonPressed :type "Key Structure"))
  (bind _asbp_character (cast `/Game/BluePrint/Character/BP_Character` (`GameplayStatics.GetPlayerCharacter` 0)))
  (if (<= (`KismetMathLibrary.Vector_Distance` (`self.K2_GetActorLocation`) (`self.K2_GetActorLocation` _asbp_character)) 500.0)
    (bind _asplayer_controller (cast `/Game/BluePrint/Character/PlayerController` (`GameplayStatics.GetPlayerController` 0)))
    (bind _getitem (`/Game/BluePrint/Character/PlayerController.ItemGet` _asplayer_controller (`self.ItemObject`)))
    (if _getitem
      (`self.K2_DestroyActor`))))

(fn `UserConstructionScript`)
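; Player controller that holds the character's inventory and equipment maps, seeding the inventory with sword and staff rows from ItemTable at BeginPlay.
; ItemGet fills the first free slot up to MaxItemCount, while DropItem spawns a BP_Item at the character's location.
; changeWeapon pushes the equipped weapon's AnimBP, mesh and attack or magic power to BP_Character, plus the accessory's element.
; Axe currently shares the Wizard branch.
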(event `self.ReceiveBeginPlay`
  (`|ExecutionSequence`
    (:`then_0`
      (bind _returnvalue (`|GetDataTableRow` "/Game/BluePrint/Inventory/ItemTable.ItemTable" "Sword")
        (:`then`
          (`BlueprintMapLibrary.Map_Add` (`self.ItemMap`) 0 _returnvalue)
          (bind _returnvalue_2 (`|GetDataTableRow` "/Game/BluePrint/Inventory/ItemTable.ItemTable" "staff")
            (:`then`
              (`BlueprintMapLibrary.Map_Add` (`self.ItemMap`) 1 _returnvalue_2))))))))

(event `DropItem`
  (params (Item :type "/Game/BluePrint/Item/SItemStruct Structure"))
  (bind _asbp_character (cast `/Game/BluePrint/Character/BP_Character` (`GameplayStatics.GetPlayerCharacter` 0)))
  (`|SpawnActorFromClass` "/Game/BluePrint/Item/BP_Item.BP_Item_C" (`KismetMathLibrary.MakeTransform` (`self.K2_GetActorLocation` _asbp_character)) "AlwaysSpawn" "OverrideRootScale" null Item null))

(event `changeWeapon`
  (bind _as_bp_character (`self.As BP Character`))
  (bind _value (`BlueprintMapLibrary.Map_Find` (`self.EquipMap`) "NewEnumerator0"))
  ;[1 1 1] 무기가 변경되었을 때 애니메이션 블루프린트를 교체한다.
  (`|ExecutionSequence`
    (:`then_0`
      (bind _asbp_character (cast `/Game/BluePrint/Character/BP_Character` (`self.K2_GetPawn`)))
      (set `self.As BP Character` _asbp_character))
    (:`then_1`
      (switch `/Game/BluePrint/Item/WeaponEnum` (`.WeaponType_31_5B9515E84375CF400157BCB1342C7C1B` (break `/Game/BluePrint/Item/SItemStruct` _value))
        (:`NewEnumerator3`
          (set `self.Anim BP` "/Game/Mannequin/Animations/ThirdPerson_AnimBP.ThirdPerson_AnimBP_C"))
        (:`NewEnumerator0`
          (set `self.Anim BP` "/Game/Animation/Player/Sword/SwordAnim.SwordAnim_C")
          (`CharacterBase.ChangeAttackMagic` _as_bp_character 0.0)
          (`CharacterBase.ChangeAttackPower` _as_bp_character (`.Value_26_338D21DA4F0FA6B964D15F84D2EDB37A` (break `/Game/BluePrint/Item/SItemStruct` _value))))
        (:`NewEnumerator1`
          (set `self.Anim BP` "/Game/Animation/Player/Wizard/AB_Wizard.AB_Wizard_C" :!label _label)
          (`CharacterBase.ChangeAttackMagic` _as_bp_character (`.Value_26_338D21DA4F0FA6B964D15F84D2EDB37A` (break `/Game/BluePrint/Item/SItemStruct` _value)))
          (`CharacterBase.ChangeAttackPower` _as_bp_character 0.0))
        (:`NewEnumerator2`
          (goto _label)))
      (set `self.Weapon` (`.ItemStaticMesh_10_CB9A95C249FBEEE9C2DC21BF984DA3D1` (break `/Game/BluePrint/Item/SItemStruct` _value)))
      (`/Game/BluePrint/Character/BP_Character.AnimChange` _as_bp_character (`self.Anim BP`) (`self.Weapon`) (`.WeaponType_31_5B9515E84375CF400157BCB1342C7C1B` (break `/Game/BluePrint/Item/SItemStruct` _value))))
    (:`then_3`
      (`/Game/BluePrint/Character/BP_Character.ChangeElement` (`self.As BP Character`) (`.AccessorieType_37_A0CBBE6B4CCE9AD31EB7C5BA98AA4D60` (break `/Game/BluePrint/Item/SItemStruct` (`BlueprintMapLibrary.Map_Find` (`self.EquipMap`) "NewEnumerator2")))))))

(fn `ItemGet`
  (params (ItemData :type "/Game/BluePrint/Item/SItemStruct Structure"))
  (returns (GetItem :type Boolean))
  (locals (Complete :type Boolean))
  (bind _itemmap (`self.ItemMap`))
  (if (>= (`BlueprintMapLibrary.Map_Length` (`self.ItemMap`)) (`self.MaxItemCount`))
    (return false)
    (else
      (for _index (range (+ (`self.MaxItemCount`) 1))
        (if (not (`.ReturnValue` (`BlueprintMapLibrary.Map_Find` _itemmap _index)))
          (`BlueprintMapLibrary.Map_Add` _itemmap _index ItemData)
          (set `local.Complete` true)
          (break)))
      (return (`local.Complete`)))))

(fn `UserConstructionScript`)
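; Player HUD Blueprint that manages the main gameplay widget and the screens shown on character and boss death.
; BeginPlay and Possess share a DoOnce that creates the main widget, and character death resets it so a later possess can rebuild the UI.
; Both death events remove the main widget and add their own screen, while other events forward visibility and weapon texture changes to the main widget.
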(event `CharacterDeath`
  (bind _returnvalue (`|CreateWidget` "/Game/BluePrint/UI/WB_Death.WB_Death_C"))
  (`UserWidget.AddToViewport` _returnvalue 0)
  (`Widget.RemoveFromParent` (`self.WB_Main`))
  (goto _label :!via `Reset`))

(event `Possess`
  (`/Engine/EditorBlueprintResources/StandardMacros.DoOnce` false :!label _label
    (:`Completed`
      (bind _returnvalue (`|CreateWidget` "/Game/BluePrint/UI/WB_Main.WB_Main_C"))
      (bind _output_get (set `self.WB_Main` _returnvalue))
      (`UserWidget.AddToViewport` _output_get 0))))

(event `self.ReceiveBeginPlay`
  (goto _label))

(event `VisibleWidget`
  (params (InVisibility :type "ESlateVisibility Enum" :default "Visible"))
  (`Widget.SetVisibility` (`self.WB_Main`) InVisibility))

(event `ChangeWeapon`
  (params (Texture :type "Texture2D Object Reference"))
  (`/Game/BluePrint/UI/WB_Main.ChangeWeapon` (`self.WB_Main`) Texture))

(event `BossDeath`
  (bind _returnvalue (`|CreateWidget` "/Game/BluePrint/UI/WB_BossDeath.WB_BossDeath_C"))
  (`UserWidget.AddToViewport` _returnvalue 0)
  (`Widget.RemoveFromParent` (`self.WB_Main`)))

(fn `UserConstructionScript`)
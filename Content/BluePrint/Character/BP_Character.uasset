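; Player character Blueprint that turns toward the mouse cursor while locally controlled, alive and outside the inventory.
; Attacks activate Gameplay Ability System abilities by tag, chosen by weapon type and, for Wizard, element, which also selects the sword trail particle.
; A scene capture shows only body and weapon for the inventory view.
; AnimChange swaps anim class, weapon mesh and type; Death disables input and collision, then triggers the sword death ability.
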(event `self.ReceiveTick`
  (params (DeltaSeconds :type "Float (single-precision)"))
  (bind _returnvalue (`self.K2_GetActorRotation`))
  (bind _returnvalue_2 (`self.K2_GetActorLocation`))
  (bind (_worldlocation _worlddirection) (`PlayerController.DeprojectMousePositionToWorld` (`GameplayStatics.GetPlayerController` 0)))
  ;[1 1 1] tick 중복호출 및 시퀀스 테스트
  (`|ExecutionSequence`
    (:`then_0`
      (if (and (`self.IsLocallyControlled`) (not (`CPP_CharacterController.bInventory` (cast `/Game/BluePrint/Character/PlayerController` (`GameplayStatics.GetPlayerController` 0) :!pure true))) (`self.bIsAlive`))
        (`self.K2_SetActorRotation` (`KismetMathLibrary.RInterpTo` _returnvalue (`KismetMathLibrary.RLerp` _returnvalue (`KismetMathLibrary.FindLookAtRotation` _returnvalue_2 (`KismetMathLibrary.MakeVector` (.x (+ _worldlocation (* _worlddirection (`SpringArmComponent.TargetArmLength` (`self.SpringArm`))))) (.y (+ _worldlocation (* _worlddirection (`SpringArmComponent.TargetArmLength` (`self.SpringArm`))))) (.z _returnvalue_2))) 1.0 true) DeltaSeconds 20.0))))))

(event `SetSceneCapture`
  (bind _scenecapturecomponent2d (`self.SceneCaptureComponent2D`))
  ;[1 1 1] 인벤토리창에 무기와 몸체만 보이도록 설정
  (`SceneCaptureComponent.ClearShowOnlyComponents` _scenecapturecomponent2d)
  (`SceneCaptureComponent.ShowOnlyComponent` _scenecapturecomponent2d (`self.Mesh`))
  (`SceneCaptureComponent.ShowOnlyComponent` (`self.SceneCaptureComponent2D`) (`self.Weapon`)))

(event `self.ReceiveBeginPlay`
  (`self.SetSceneCapture`)
  (`self.ChangeElement` "Aqua"))

(event `InputAction|Attack`
  (params (Key :type "Key Structure"))
  (bind _abilitysystemcomp (`self.AbilitySystemComp`))
  ;[1 1 1] 공격 (GameplayAbility를 이용해 몽타주를 전역에 뿌림)
  (:`Pressed`
    (switch `/Game/BluePrint/Item/WeaponEnum` (`self.Weapon Type`)
      (:`NewEnumerator0`
        (`GASComponent.TryActiveAbilitiesByTagAndReturn` _abilitysystemcomp (`self.SwordAttack Tag Container`) true)
        (set `self.CoolDownEffect` "/Game/BluePrint/GAS/Character/GE_CoolDown.GE_CoolDown_C"))
      (:`NewEnumerator1`
        (switch `EElementEnum` (`self.Element`)
          (:`None`
            (`GASComponent.TryActiveAbilitiesByTagAndReturn` _abilitysystemcomp (`self.WizardFire Tag Container`) true :!label _label))
          (:`Fire`
            (goto _label))
          (:`Aqua`
            (`GASComponent.TryActiveAbilitiesByTagAndReturn` _abilitysystemcomp (`self.WizardAqua Tag Container`) true))
          (:`Lightning`
            (`GASComponent.TryActiveAbilitiesByTagAndReturn` _abilitysystemcomp (`self.WizardLightning Tag Container`) true)))
        (set `self.CoolDownEffect` "/Game/BluePrint/GAS/Character/Wizard/GE_WizardCoolDown.GE_WizardCoolDown_C")))))

(event `ChangeElement`
  (params (Element :type "EElementEnum Enum" :default "None"))
  ;[1 1 1] 장신구를 교체시 파티클을 변경. 후에 추가되거나 변경 예정
  (bind _output_get (set `self.Element` Element))
  (switch `EElementEnum` _output_get
    (:`None`
      (set `self.SwordTrailElement` "/Game/Animation/Player/Sword/SwordTrail_Fire.SwordTrail_Fire" :!label _label_2))
    (:`Fire`
      (goto _label_2))
    (:`Aqua`
      (set `self.SwordTrailElement` "/Game/Animation/Player/Sword/SwordTrail_Aqua.SwordTrail_Aqua"))
    (:`Lightning`
      (set `self.SwordTrailElement` "/Game/Animation/Player/Sword/SwordTrail_Thunder.SwordTrail_Thunder"))))

(event `self.Death`
  ;[1 1 1] 애니메이션 마다 Death 어빌리티를 작성해서 불러와야함 나중에 수정 예정
  (`self.DisableInput` null)
  (set `self.bIsAlive` false)
  (`PrimitiveComponent.SetCollisionEnabled` (`self.Mesh`) "NoCollision")
  (`PrimitiveComponent.SetCollisionEnabled` (`self.CapsuleComponent`) "NoCollision")
  (`PrimitiveComponent.SetCollisionEnabled` (`self.Weapon`) "NoCollision")
  (`AbilitySystemComponent.TryActivateAbilitiesByTag` (`AbilitySystemBlueprintLibrary.GetAbilitySystemComponent` self) (`self.SwordDeath Tag Container`) true))

(event `AnimChange_Implement`
  (params (AnimBlueprint :type "AnimInstance Class Reference") (Weapon :type "StaticMesh Object Reference") (WeaponType :type "/Game/BluePrint/Item/WeaponEnum Enum" :default "NewEnumerator3"))
  (`SkeletalMeshComponent.SetAnimInstanceClass` (`self.Mesh`) AnimBlueprint)
  (`StaticMeshComponent.SetStaticMesh` (`self.Weapon`) Weapon)
  (set `self.Weapon Type` WeaponType))

(event `AnimChange`
  (params (AnimBlueprint :type "AnimInstance Class Reference") (Weapon :type "StaticMesh Object Reference") (WeaponType :type "/Game/BluePrint/Item/WeaponEnum Enum" :default "NewEnumerator3"))
  (`self.AnimChange_Implement` AnimBlueprint Weapon WeaponType))

(fn `UserConstructionScript`)
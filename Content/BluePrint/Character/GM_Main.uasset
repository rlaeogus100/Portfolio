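; Game mode that runs enemy spawning and player respawn around the first Start1 actor.
; A Tick-driven DoOnce and five-second Delay loop spawns random batches of AI trolls while few remain and the boss kill threshold is not exceeded.
; Reaching that threshold spawns Enemy_Boss once.
; A bound respawn event spawns and possesses a new BP_Character, while CountReturn and BeginPlay copy kill counts to all PlayerControllers.
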(event `CountReturn`
  (bind _outactors (`GameplayStatics.GetAllActorsOfClass` "/Game/BluePrint/Character/PlayerController.PlayerController_C" :!label _label))
  (for _array_element _outactors
    (set `/Game/BluePrint/Character/PlayerController.MonsterKill` (`self.MonsterKillCount`) _array_element)
    (set `/Game/BluePrint/Character/PlayerController.BossSpawn` (`self.BossSpawnCount`) _array_element)))

(event `self.ReceiveBeginPlay`
  (add `self.RespawnPlayer` (delegate `NewEventDispatcher_0_Event`))
  (goto _label))

(event `NewEventDispatcher_0_Event` :!signature `self.RespawnPlayer`
  (params (NewParam :type "/Game/BluePrint/Character/PlayerController Object Reference"))
  (bind _outactors (`GameplayStatics.GetAllActorsOfClass` "/Game/BluePrint/Character/Start1.Start1_C"))
  (bind _returnvalue (`|SpawnActorFromClass` "/Game/BluePrint/Character/BP_Character.BP_Character_C" (`self.GetTransform` (`|GetArrayItem` _outactors)) "AdjustIfPossibleButAlwaysSpawn" "OverrideRootScale" NewParam null))
  (`Controller.Possess` NewParam _returnvalue))

(event `self.ReceiveTick`
  (params (DeltaSeconds :type "Float (single-precision)"))
  (`|ExecutionSequence`
    (:`then_0`
      (`/Engine/EditorBlueprintResources/StandardMacros.DoOnce` false :!label _label_2
        (:`Completed`
          (`self.GM Spawn Actor`)
          (`KismetSystemLibrary.Delay` 5.0)
          (goto _label_2 :!via `Reset`))))
    (:`then_1`
      (if (>= (`self.MonsterKillCount`) (`self.BossSpawnCount`))
        (`/Engine/EditorBlueprintResources/StandardMacros.DoOnce` false
          (:`Completed`
            (bind _outactors (`GameplayStatics.GetAllActorsOfClass` "/Game/BluePrint/Character/Start1.Start1_C"))
            (bind _returnvalue (`self.GetTransform` (`|GetArrayItem` _outactors)))
            (`AIBlueprintHelperLibrary.SpawnAIFromClass` "/Game/BluePrint/Enemy/Enemy_Boss.Enemy_Boss_C" "/Game/BluePrint/Enemy/BT_Enemy.BT_Enemy" (`KismetMathLibrary.MakeVector` (.x (.location _returnvalue)) (.y (.location _returnvalue)) (+ (.z (.location _returnvalue)) 100.0)) (.rotation _returnvalue) false null)))))))

(event `GM Spawn Actor`
  (bind _returnvalue (`KismetMathLibrary.RandomFloatInRange` -100.0 100.0))
  (bind _outactors (`GameplayStatics.GetAllActorsOfClass` "/Game/BluePrint/Enemy/Enemy_Troll.Enemy_Troll_C"))
  (if (and (<= (`self.MonsterKillCount`) (`self.BossSpawnCount`)) (<= (`KismetArrayLibrary.Array_Length` _outactors) 2))
    (bind _outactors_2 (`GameplayStatics.GetAllActorsOfClass` "/Game/BluePrint/Character/Start1.Start1_C"))
    (for _ (range (+ (`KismetMathLibrary.RandomInteger` 7) 1))
      (bind _returnvalue_2 (`self.GetTransform` (`|GetArrayItem` _outactors_2)))
      (`AIBlueprintHelperLibrary.SpawnAIFromClass` "/Game/BluePrint/Enemy/Enemy_Troll.Enemy_Troll_C" "/Game/BluePrint/Enemy/BT_Enemy.BT_Enemy" (`KismetMathLibrary.MakeVector` (+ (.x (.location _returnvalue_2)) _returnvalue) (+ (.y (.location _returnvalue_2)) _returnvalue) (.z (.location _returnvalue_2))) (.rotation _returnvalue_2) false null))))

(fn `UserConstructionScript`)